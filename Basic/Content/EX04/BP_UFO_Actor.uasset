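; UFO actor exercise that spins continuously around the roll, pitch or yaw axis chosen by Type.
; Tick caches delta time and calls one of six helpers, using local rotation offsets; unused SetActorRotation versions remain, one noted as buggy.
; T, G, H and F set MoveType, but Tick never reads it.
; Only forward movement exists, along world X, reached through a switch on Move_Foward_T under Roll Plus.
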(event EventTick
  (params (DeltaSeconds :type Float%20%28single-precision%29))
  (Variables|Default|SetActorDeltaSecond DeltaSeconds)
  (switch Utilities|FlowControl|Switch|SwitchonE_Rotation (Variables|Default|GetType)
    (:NewEnumerator0
      (CallFunction|RollPlus)
      (switch Utilities|FlowControl|Switch|SwitchonE_Location "NewEnumerator0"
        (:NewEnumerator0
          (CallFunction|MoveFoward))))
    (:NewEnumerator1
      (CallFunction|RollMinus))
    (:NewEnumerator2
      (CallFunction|PitchPlus))
    (:NewEnumerator3
      (CallFunction|PitchMinus))
    (:NewEnumerator4
      (CallFunction|YawPlus))
    (:NewEnumerator5
      (CallFunction|YawMinus))))

(event Input|KeyboardEvents|F
  (params (Key :type Key%20Structure :default "None"))
  (:Pressed
    (Variables|Default|SetMoveType "NewEnumerator3")))

(event Input|KeyboardEvents|T
  (params (Key :type Key%20Structure :default "None"))
  (:Pressed
    (Variables|Default|SetMoveType "NewEnumerator0")))

(event Input|KeyboardEvents|G
  (params (Key :type Key%20Structure :default "None"))
  (:Pressed
    (Variables|Default|SetMoveType "NewEnumerator1")))

(event Input|KeyboardEvents|H
  (params (Key :type Key%20Structure :default "None"))
  (:Pressed
    (Variables|Default|SetMoveType "NewEnumerator2")))

(fn ConstructionScript)

(fn RollPlus
  (Transformation|AddActorLocalRotation (Math|Rotator|MakeRotator (* (Variables|Default|GetRotationSpeed) (Variables|Default|GetActorDeltaSecond)) 0.0 0.0) false false))

(fn RollMinus
  (Transformation|AddActorLocalRotation (Math|Rotator|MakeRotator (* (* (Variables|Default|GetRotationSpeed) (Variables|Default|GetActorDeltaSecond)) -1.0) 0.0 0.0) false false))

(fn PitchPlus
  (Transformation|AddActorLocalRotation (Math|Rotator|MakeRotator 0.0 (* (Variables|Default|GetRotationSpeed) (Variables|Default|GetActorDeltaSecond)) 0.0) false false))

(fn PitchMinus
  (Transformation|AddActorLocalRotation (Math|Rotator|MakeRotator 0.0 (* (* (Variables|Default|GetRotationSpeed) (Variables|Default|GetActorDeltaSecond)) -1.0) 0.0) false false))

(fn YawPlus
  (Transformation|AddActorLocalRotation (Math|Rotator|MakeRotator 0.0 0.0 (* (Variables|Default|GetRotationSpeed) (Variables|Default|GetActorDeltaSecond))) false false))

(fn YawMinus
  (Transformation|AddActorLocalRotation (Math|Rotator|MakeRotator 0.0 0.0 (* (* (Variables|Default|GetRotationSpeed) (Variables|Default|GetActorDeltaSecond)) -1.0)) false false))

(fn MoveFoward
  (bind _returnvalue (Transformation|GetActorLocation))
  (Transformation|SetActorLocation (Math|Vector|MakeVector (+ (.x _returnvalue) (* (Variables|Default|GetMoveSpeed) (Variables|Default|GetActorDeltaSecond))) (.y _returnvalue) (.z _returnvalue)) false false))