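; Game state for the EX05 exercise that holds a coin count and changes level when the coins run out.
; DecreaseCoinCount lowers the count while it is above zero and pushes the new value to the coin info UMG widget.
; At zero it opens L_EX05, but only if that widget reference is valid, since the level check follows the widget update.
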(fn ConstructionScript)

(fn GetCoin
  (return (Variables|Default|GetCoinCount)))

(fn DecreaseCoinCount
  (if (> (Variables|Default|GetCoinCount) 0)
    (Variables|Default|SetCoinCount (- (Variables|Default|GetCoinCount) 1))
    (Utilities|IsValid (Variables|Default|GetUMGCoin%20Info)
      (:Is%20Valid
        (Default|SetRemainCoinCount (Variables|Default|GetUMGCoin%20Info) (Variables|Default|GetCoinCount))
        (if (<= (Variables|Default|GetCoinCount) 0)
          (Game|OpenLevel(byObjectReference) "/Game/EX05/L_EX05.L_EX05"))))))