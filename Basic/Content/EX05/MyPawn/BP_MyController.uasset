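; BP_MyController is a player controller that drives the controlled pawn through Enhanced Input, adding IMC_MyPawn on BeginPlay.
; Move input becomes movement along directions derived from control rotation, and look input feeds controller yaw and pitch.
; Holding jump flies the pawn by directly offsetting its Z location by negated FlySpeed times Tick's delta seconds, bypassing movement input.
; An up-vector movement input node remains unconnected.
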(event Input|EnhancedActionEvents|EnhancedInputActionIA_MovePawn
  (params (ActionValue :type Vector%202D%20Structure) (ElapsedSeconds :type Float%20%28double-precision%29) (TriggeredSeconds :type Float%20%28double-precision%29) (InputAction :type Input%20Action%20Object%20Reference :default "/Game/EX05/MyPawn/Input/IA_MovePawn.IA_MovePawn"))
  (bind _returnvalue (Pawn|GetControlledPawn))
  (bind _returnvalue_2 (Pawn|GetControlRotation :!class /Script/Engine.Controller))
  (Pawn|Input|AddMovementInput _returnvalue (Math|Vector|GetRightVector (Math|Rotator|MakeRotator (.roll _returnvalue_2) 0.0 (.yaw _returnvalue_2))) (.x ActionValue) false)
  (Pawn|Input|AddMovementInput _returnvalue (Math|Vector|GetForwardVector (Math|Rotator|MakeRotator 0.0 0.0 (.yaw (Pawn|GetControlRotation :!class /Script/Engine.Controller)))) (.y ActionValue) false))

(event Input|EnhancedActionEvents|EnhancedInputActionIA_LookPawn
  (params (ActionValue :type Vector%202D%20Structure) (ElapsedSeconds :type Float%20%28double-precision%29) (TriggeredSeconds :type Float%20%28double-precision%29) (InputAction :type Input%20Action%20Object%20Reference :default "/Game/EX05/MyPawn/Input/IA_LookPawn.IA_LookPawn"))
  (bind _returnvalue (Pawn|GetControlledPawn))
  (Pawn|Input|AddControllerYawInput _returnvalue (.x ActionValue))
  (Pawn|Input|AddControllerPitchInput _returnvalue (.y ActionValue)))

(event Input|EnhancedActionEvents|EnhancedInputActionIA_JumpPawn
  (params (ActionValue :type Float%20%28double-precision%29) (ElapsedSeconds :type Float%20%28double-precision%29) (TriggeredSeconds :type Float%20%28double-precision%29) (InputAction :type Input%20Action%20Object%20Reference :default "/Game/EX05/MyPawn/Input/IA_JumpPawn.IA_JumpPawn"))
  (bind _returnvalue (Pawn|GetControlledPawn))
  (bind _returnvalue_2 (Transformation|GetActorLocation _returnvalue))
  ;[1 1 1] Press 'Space bar' Pawn is flying
  (:Triggered
    (Transformation|SetActorLocation _returnvalue (Math|Vector|MakeVector (.x _returnvalue_2) (.y _returnvalue_2) (+ (.z _returnvalue_2) (* (* (Variables|Default|GetFlySpeed) (stale EventTick DeltaSeconds)) -1.0))) false false)))

(event EventBeginPlay
  (Input|AddMappingContext (PlayerController|LocalPlayerSubsystems|GetEnhancedInputLocalPlayerSubsystem) "/Game/EX05/MyPawn/Input/IMC_MyPawn.IMC_MyPawn" 0 "(bIgnoreAllPressedKeysUntilRelease=True,bForceImmediately=False,bNotifyUserSettings=False)"))

(event EventTick
  (params (DeltaSeconds :type Float%20%28single-precision%29))
  ;[1 1 1] Press 'Space bar' Pawn is flying
)

(fn ConstructionScript)