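; BP_DynamicActor is a glowing mesh actor that changes color while the player's BP_MyPawn is inside its trigger box.
; On BeginPlay it creates a dynamic instance of M_DynamicGlow on the mesh and applies its variables for glow color, frequency, intensity, metallic and roughness.
; Trigger overlap begin switches the GlowOrbColor parameter to ColorValue, and overlap end restores BeginColor, reacting only to BP_MyPawn.
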(event OnComponentBeginOverlap(TriggerBox)
  (params (OverlappedComponent :type Primitive%20Component%20Object%20Reference) (OtherActor :type Actor%20Object%20Reference) (OtherComp :type Primitive%20Component%20Object%20Reference) (OtherBodyIndex :type Integer) (bFromSweep :type Boolean) (SweepResult :type Hit%20Result%20Structure%20%28by%20ref%29))
  (Utilities|Casting|CastToBP_MyPawn OtherActor)
  (Rendering|Material|SetVectorParameterValue (Variables|Default|GetDynamicMaterial) "GlowOrbColor" (Variables|Default|GetColorValue) :!class /Script/Engine.MaterialInstanceDynamic))

(event OnComponentEndOverlap(TriggerBox)
  (params (OverlappedComponent :type Primitive%20Component%20Object%20Reference) (OtherActor :type Actor%20Object%20Reference) (OtherComp :type Primitive%20Component%20Object%20Reference) (OtherBodyIndex :type Integer))
  (Utilities|Casting|CastToBP_MyPawn OtherActor)
  (Rendering|Material|SetVectorParameterValue (Variables|Default|GetDynamicMaterial) "GlowOrbColor" (Variables|Default|GetBeginColor) :!class /Script/Engine.MaterialInstanceDynamic))

(event EventBeginPlay
  (bind _returnvalue (Rendering|Material|CreateDynamicMaterialInstance (Variables|Default|GetStaticMesh) 0 "/Game/EX02/M_DynamicGlow.M_DynamicGlow" "None" :!class /Script/Engine.PrimitiveComponent))
  (bind _output_get (Variables|Default|SetDynamicMaterial _returnvalue))
  (Utilities|FlowControl|Sequence
    (:then_0
      (Rendering|Material|SetVectorParameterValue _output_get "GlowOrbColor" (Variables|Default|GetBeginColor) :!class /Script/Engine.MaterialInstanceDynamic))
    (:then_1
      (Rendering|Material|SetScalarParameterValue _output_get "Frequency" (Variables|Default|GetFrequencyValue) :!class /Script/Engine.MaterialInstanceDynamic))
    (:then_2
      (Rendering|Material|SetScalarParameterValue _output_get "Intensity" (Variables|Default|GetIntensityValue) :!class /Script/Engine.MaterialInstanceDynamic))
    (:then_3
      (Rendering|Material|SetScalarParameterValue _output_get "Metallic" (Variables|Default|GetMetallicValue) :!class /Script/Engine.MaterialInstanceDynamic))
    (:then_4
      (Rendering|Material|SetScalarParameterValue _output_get "Roughness" (Variables|Default|GetRoughnessValue) :!class /Script/Engine.MaterialInstanceDynamic))))

(fn ConstructionScript)