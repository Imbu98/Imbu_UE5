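; BP_Projectile is a projectile actor that fires forward when Launch is called and destroys itself after a few seconds.
; Launch applies a velocity-change impulse to the static mesh along the actor's forward vector, then starts a timer by function name for DestroyProjectile.
; It also calls BulletColor, which creates a dynamic chrome material instance and gives its color parameter random values on each launch.
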(event EventBeginPlay)

(event EventTick
  (params (DeltaSeconds :type Float%20%28single-precision%29)))

(fn ConstructionScript)

(fn Launch
  (Physics|AddImpulse (Variables|Default|GetStaticMesh) (* (Transformation|GetActorForwardVector) 1e+04) "None" true)
  (CallFunction|BulletColor)
  (Utilities|Time|SetTimerbyFunctionName 0 "DestroyProjectile" 3.0))

(fn DestroyProjectile
  (Actor|DestroyActor))

(fn BulletColor
  (bind _returnvalue (Rendering|Material|CreateDynamicMaterialInstance (Variables|Default|GetStaticMesh) 0 "/Game/_Asset/Material/M_Metal_Chrome.M_Metal_Chrome" "None" :!class /Script/Engine.PrimitiveComponent))
  (bind _output_get (Variables|Default|SetBulletMaterial _returnvalue))
  (Rendering|Material|SetVectorParameterValue _output_get "BulletColor" (Utilities|Struct|MakeLinearColor (Math|Random|RandomFloat) (Math|Random|RandomFloat) (Math|Random|RandomFloat) (Math|Random|RandomFloat)) :!class /Script/Engine.MaterialInstanceDynamic))