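; BP_GC_Sphere is a sphere actor that spins until a projectile hits it, then removes itself.
; Tick rotates it in local pitch at LotateSpeed, scaled by delta time, while Overlap is false.
; The first BP_Projectile overlap sets Overlap, halting rotation, and starts a three-second timer that destroys the actor and sets IsDestroyed.
; A SpawnSphere function, not called here, spawns another copy far along X from its location.
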(event OnComponentBeginOverlap(Sphere)
  (params (OverlappedComponent :type Primitive%20Component%20Object%20Reference) (OtherActor :type Actor%20Object%20Reference) (OtherComp :type Primitive%20Component%20Object%20Reference) (OtherBodyIndex :type Integer) (bFromSweep :type Boolean) (SweepResult :type Hit%20Result%20Structure%20%28by%20ref%29))
  (if (not (Variables|Default|GetOverlap))
    (Utilities|Casting|CastToBP_Projectile OtherActor)
    (Variables|Default|SetOverlap true)
    (Utilities|Time|SetTimerbyEvent (delegate Custom|커스텀이벤트) 3.0)))

(event Custom|커스텀이벤트
  (Actor|DestroyActor)
  (Variables|Default|SetIsDestroyed true))

(event EventBeginPlay)

(event EventTick
  (params (DeltaSeconds :type Float%20%28single-precision%29))
  (if (not (Variables|Default|GetOverlap))
    (Transformation|AddActorLocalRotation (Math|Rotator|MakeRotator 0.0 (* DeltaSeconds (Variables|Default|GetLotateSpeed)) 0.0) false false)))

(fn ConstructionScript)

(fn SpawnSphere
  (Game|SpawnActorfromClass "BP_GC_Sphere_C" (Math|Transform|MakeTransform (Math|Vector|MakeVector (+ 1e+04 (.x (Transformation|GetActorLocation))) 0.0 0.0) "0, 0, 0" "1.000000,1.000000,1.000000") "Undefined" "MultiplyWithRoot" 0 0))