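; BP_Actor02_Dynamic is an actor that gives its static mesh a configurable glowing look at runtime.
; On BeginPlay it creates a dynamic material instance of M_DynamicGlow on the mesh's first material slot and stores it.
; It then copies the actor's color, frequency, intensity, metallic and roughness variables into the matching material parameters, with no later updates in this graph.
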(event EventBeginPlay
  (bind _returnvalue (Rendering|Material|CreateDynamicMaterialInstance (Variables|Default|GetStaticMesh) 0 "/Game/EX02/M_DynamicGlow.M_DynamicGlow" "None" :!class /Script/Engine.PrimitiveComponent))
  (bind _output_get (Variables|Default|SetDynamicMaterial _returnvalue))
  (Utilities|FlowControl|Sequence
    (:then_0
      (Rendering|Material|SetVectorParameterValue _output_get "GlowOrbColor" (Variables|Default|GetColorValue) :!class /Script/Engine.MaterialInstanceDynamic))
    (:then_1
      (Rendering|Material|SetScalarParameterValue _output_get "Frequency" (Variables|Default|GetFrequencyValue) :!class /Script/Engine.MaterialInstanceDynamic))
    (:then_2
      (Rendering|Material|SetScalarParameterValue _output_get "Intensity" (Variables|Default|GetIntensityValue) :!class /Script/Engine.MaterialInstanceDynamic))
    (:then_3
      (Rendering|Material|SetScalarParameterValue _output_get "Metallic" (Variables|Default|GetMetallicValue) :!class /Script/Engine.MaterialInstanceDynamic))
    (:then_4
      (Rendering|Material|SetScalarParameterValue _output_get "Roughness" (Variables|Default|GetRoughnessValue) :!class /Script/Engine.MaterialInstanceDynamic))))

(fn ConstructionScript)