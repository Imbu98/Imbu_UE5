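; BP_EX03_2 is an exercise actor that moves continuously along world X or Y according to its current direction state.
; Each Tick switches on CurrentDir: T/G move along ±X and H/F along ±Y, scaled by MoveValue and delta time, while Space calls SetActorLocation with default inputs.
; MoveActor stores the incoming direction and flags ChangeDir when it differs; nothing here reads that flag.
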(event EventTick
  (params (DeltaSeconds :type Float%20%28single-precision%29))
  (bind _returnvalue (Transformation|GetActorLocation))
  (bind _returnvalue_2 (Transformation|GetActorLocation))
  (Variables|Default|SetDelta%20Seconds DeltaSeconds)
  (switch Utilities|FlowControl|Switch|SwitchonDirection (Variables|Default|GetCurrentDir)
    (:NewEnumerator0
      (Transformation|SetActorLocation (Math|Vector|MakeVector (+ (.x _returnvalue) (* (Variables|Default|GetDelta%20Seconds) (Variables|Default|GetMoveValue))) (.y _returnvalue) 0.0) false false))
    (:NewEnumerator1
      (Transformation|SetActorLocation (Math|Vector|MakeVector (+ (.x _returnvalue) (* (* (Variables|Default|GetDelta%20Seconds) (Variables|Default|GetMoveValue)) -1.0)) (.y _returnvalue) 0.0) false false))
    (:NewEnumerator2
      (Transformation|SetActorLocation (Math|Vector|MakeVector (.x _returnvalue_2) (+ (.y _returnvalue_2) (* (* (Variables|Default|GetDelta%20Seconds) (Variables|Default|GetMoveValue)) -1.0)) 0.0) false false))
    (:NewEnumerator3
      (Transformation|SetActorLocation (Math|Vector|MakeVector (.x _returnvalue_2) (+ (.y _returnvalue_2) (* (Variables|Default|GetDelta%20Seconds) (Variables|Default|GetMoveValue))) 0.0) false false))
    (:NewEnumerator4
      (Transformation|SetActorLocation (Math|Vector|MakeVector 0.0 0.0 0.0) false false))))

(fn ConstructionScript)

(fn MoveActor
  (params (inDir :type Direction%20Enum :default "NewEnumerator0"))
  (if (Utilities|Enum|NotEqual(Enum) inDir (Variables|Default|GetCurrentDir))
    (Variables|Default|SetChangeDir true)
    (else
      (Variables|Default|SetChangeDir false)))
  (Variables|Default|SetCurrentDir inDir))